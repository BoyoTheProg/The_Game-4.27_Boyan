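; BP_FloorTile is a floor segment for a runner game that extends the track as the player moves along it.
; On construction it stores three spawn point transforms and adds an obstacle child actor at a randomly chosen one.
; When a BP_RunCharacter overlaps ExitBox, it calls ExtendFloor on BP_RunnerGameMode.
; GetAttachPoint exposes the AttachPoint world transform.
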(event `self.ExitBox.OnComponentBeginOverlap`
  (params (OverlappedComponent :type "PrimitiveComponent Object Reference") (OtherActor :type "Actor Object Reference") (OtherComp :type "PrimitiveComponent Object Reference") (OtherBodyIndex :type Integer) (bFromSweep :type Boolean) (SweepResult :type "HitResult Structure (by ref)"))
  (cast `/Game/Runner/Blueprints/BP_RunCharacter` OtherActor)
  (bind _asbp_runner_game_mode (cast `/Game/Runner/Blueprints/BP_RunnerGameMode` (`GameplayStatics.GetGameMode`)))
  (`/Game/Runner/Blueprints/BP_RunnerGameMode.ExtendFloor` _asbp_runner_game_mode))

(fn `GetAttachPoint`
  (returns (Value :type "Transform Structure"))
  (return (`SceneComponent.K2_GetComponentToWorld` (`self.AttachPoint`))))

(fn `SetSpawnPoints`
  (set `self.GetSpawnPoints` (`|MakeArray` (`SceneComponent.GetRelativeTransform` (`self.SpawnPointRight`)) (`SceneComponent.GetRelativeTransform` (`self.SpawnPointLeft`)) (`SceneComponent.GetRelativeTransform` (`self.SpawnPoint`)))))

(fn `SpawnObsticle`
  (bind _getspawnpoints (`self.GetSpawnPoints`))
  (`AddComponent|NODE_AddChildActorComponent-2` :`RelativeTransform` (`|GetArrayItem` _getspawnpoints (`KismetMathLibrary.RandomIntegerInRange` 0 (`KismetArrayLibrary.Array_LastIndex` _getspawnpoints)))))

(fn `UserConstructionScript`
  (`self.SetSpawnPoints`)
  (`self.SpawnObsticle`))