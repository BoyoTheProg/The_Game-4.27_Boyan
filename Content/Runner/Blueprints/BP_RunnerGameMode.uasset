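; BP_RunnerGameMode is the game mode for a runner game that builds and recycles a chain of floor tiles.
; On BeginPlay it spawns NumOfTiles BP_FloorTile actors end to end, each at the previous tile's attach point, tracking them in the FloorTile array.
; ExtendFloor adds a tile and destroys the oldest once the array exceeds NumOfTiles + 1, keeping a rolling track of bounded length.
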(event `self.ReceiveBeginPlay`
  (for _ (range (`self.NumOfTiles`))
    (`self.AddFloor`)))

(fn `AddFloor`
  (locals (FloorTiles :type "Array of Actor Class Reference"))
  (bind _returnvalue (`|SpawnActorFromClass` "/Game/Runner/Blueprints/BP_FloorTile.BP_FloorTile_C" (`self.FloorAttachPoint`) "Undefined" "OverrideRootScale" null null))
  (set `self.FloorAttachPoint` (`/Game/Runner/Blueprints/BP_FloorTile.GetAttachPoint` _returnvalue))
  (`KismetArrayLibrary.Array_Add` (`self.FloorTile`) _returnvalue))

(fn `ExtendFloor`
  (bind _floortile (`self.FloorTile`))
  (bind _output (`|GetArrayItem` _floortile))
  (`self.AddFloor`)
  (if (> (`KismetArrayLibrary.Array_Length` (`self.FloorTile`)) (+ (`self.NumOfTiles`) 1))
    (`self.K2_DestroyActor` _output)
    (`KismetArrayLibrary.Array_RemoveItem` _floortile _output)))

(fn `UserConstructionScript`)