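; Player character for an endless-runner style game that runs forward automatically along its control yaw until it dies.
; Up or Space jumps, while Left and Right step between three lanes using a timeline that lerps the actor's Y toward the target lane.
; The Death event disables input, plays explosion effects, hides the mesh, then restarts the level by console command after a short delay.
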(event `self.ReceiveTick`
  (params (DeltaSeconds :type "Float (single-precision)"))
  (if (not (`self.Is Dead`))
    (`self.AddMovementInput` (`KismetMathLibrary.GetForwardVector` (`KismetMathLibrary.MakeRotator` 0.0 0.0 (.yaw (`self.GetControlRotation`)))))))

(event `Key|Up`
  (params (Key :type "Key Structure"))
  (:`Pressed`
    (`self.Jump` :!label _label)))

(event `Key|SpaceBar`
  (params (Key :type "Key Structure"))
  (:`Pressed`
    (goto _label)))

(event `ChangeLane`
  (params (ShiftLane :type Integer))
  (set `self.TargetLaneIndex` (`KismetMathLibrary.Clamp` (+ ShiftLane (`self.CurrentLaneIndex`)) 0 2))
  (set `self.CurrentYPosition` (.y (`self.K2_GetActorLocation`)))
  (bind (_direction _newtrack_0) (`Timeline|ChangeLaneTimeline` :!via `PlayFromStart`)
    (:`Update`
      (`self.K2_SetActorLocation` (`KismetMathLibrary.MakeVector` (.x (`self.K2_GetActorLocation`)) (`KismetMathLibrary.Lerp` (`self.CurrentYPosition`) (`|GetArrayItem` (`self.LanePositions`) (`self.TargetLaneIndex`)) _newtrack_0) (.z (`self.K2_GetActorLocation`)))))
    (:`Finished`
      (set `self.CurrentLaneIndex` (`self.TargetLaneIndex`)))))

(event `Key|Left`
  (params (Key :type "Key Structure"))
  (:`Pressed`
    (`self.ChangeLane` -1)))

(event `Death`
  (bind _returnvalue (`self.K2_GetActorLocation`))
  (set `self.Is Dead` true)
  (`self.DisableInput` null)
  (`GameplayStatics.SpawnEmitterAtLocation` "/Game/StarterContent/Particles/P_Explosion.P_Explosion" _returnvalue)
  (`GameplayStatics.PlaySoundAtLocation` "/Game/StarterContent/Audio/Explosion_Cue.Explosion_Cue" _returnvalue (struct) 1.0 1.0 0.0 null null null)
  (`SceneComponent.SetVisibility` (`self.Mesh`) false false)
  (`KismetSystemLibrary.Delay` 2.0)
  (`KismetSystemLibrary.ExecuteConsoleCommand` "RestartLevel" null))

(event `Key|Right`
  (params (Key :type "Key Structure"))
  (:`Pressed`
    (`self.ChangeLane` 1)))

(fn `UserConstructionScript`)